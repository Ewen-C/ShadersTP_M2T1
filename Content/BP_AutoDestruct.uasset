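; BP_AutoDestruct is a cube actor that plays a timed material effect and destroys itself once its box trigger is overlapped.
; The overlap creates a dynamic material instance on the cube, passing game time, DestructSpeed and a green glow so the shader animates itself without Tick.
; A timer of 1/DestructSpeed seconds then destroys the actor, matching the effect speed without actually checking transparency.
; Overlaps are not gated, and the Voronoi texture is set with parameter name None.
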(event `self.BoxTrigger.OnComponentBeginOverlap`
  (params (OverlappedComponent :type "PrimitiveComponent Object Reference") (OtherActor :type "Actor Object Reference") (OtherComp :type "PrimitiveComponent Object Reference") (OtherBodyIndex :type Integer) (bFromSweep :type Boolean) (SweepResult :type "HitResult Structure (by ref)"))
  (`|ExecutionSequence`
    (:`then_0`
      (bind _returnvalue (`KismetSystemLibrary.K2_SetTimerDelegate` (delegate `CheckMaterialTransparent`) (/ 1.0 (`self.DestructSpeed`))))
      (set `self.TimerHandle` _returnvalue))
    (:`then_1`
      (bind _returnvalue_2 (`KismetMaterialLibrary.CreateDynamicMaterialInstance` "/Game/Shaders/Rendu2_v3.Rendu2_v3"))
      (set `self.CubeMaterial` _returnvalue_2)
      (`MaterialInstanceDynamic.SetScalarParameterValue` (`self.CubeMaterial`) "EffectStartTime" (`KismetSystemLibrary.GetGameTimeInSeconds`))
      (`MaterialInstanceDynamic.SetScalarParameterValue` (`self.CubeMaterial`) "EffectSpeed" (`self.DestructSpeed`))
      (`MaterialInstanceDynamic.SetScalarParameterValue` (`self.CubeMaterial`) "StopGlowRange" 0.11)
      (`MaterialInstanceDynamic.SetVectorParameterValue` (`self.CubeMaterial`) "GlowColor" (struct :`R` 3.25 :`G` 30.0 :`A` 1.0))
      (`MaterialInstanceDynamic.SetTextureParameterValue` (`self.CubeMaterial`) "None" "/Game/Textures/voronoi_3.voronoi_3")
      (`PrimitiveComponent.SetMaterial` (`self.CubeMesh`) 0 (`self.CubeMaterial`)))))

(event `CheckMaterialTransparent`
  (`self.K2_DestroyActor`))

(fn `UserConstructionScript`)